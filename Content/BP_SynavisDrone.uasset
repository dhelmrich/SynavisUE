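; Synavis drone actor that connects Pixel Streaming to its scene and info cameras.
; Input descriptors go to ParseInput, responses return through PixelStreamingInput, and, with AutoPossess, closed connections reset Synavis state.
; Geometry events spawn a randomly rotated actor at the origin with a procedural mesh built from the received arrays.
; Signals switch the viewport between single-view and dual-view widgets for scene, info or both cameras.
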(event `self.ReceiveBeginPlay`
  (bind _returnvalue (`GameplayStatics.GetPlayerControllerFromID` 0))
  (add `self.OnPixelStreamingResponse` (delegate `OnPixelStreamingResponse_Event`))
  (add `self.OnPixelStreamingGeometry` (delegate `OnPixelStreamingGeometry_Event`))
  (add `self.OnBlueprintSignalling` (delegate `OnBlueprintSignalling_Event`))
  (bind _returnvalue_2 (`|CreateWidget` "/SynavisUE/DualViewPrint.DualViewPrint_C" _returnvalue))
  (bind _returnvalue_3 (`|CreateWidget` "/SynavisUE/SingleView.SingleView_C" _returnvalue))
  (set `self.SingleOverlay` _returnvalue_3)
  (set `self.DualOverlay` _returnvalue_2)
  (`self.SetActorHiddenInGame` (`Controller.K2_GetPawn` _returnvalue) true)
  (`ActorComponent.Activate` (`self.SceneCam`) true)
  (if (`self.AutoPossess`)
    (`self.DisableInput` (`GameplayStatics.GetPlayerPawn` 0) (`GameplayStatics.GetPlayerControllerFromID` 0))
    (`UserWidget.AddToViewport` (`self.DualOverlay`) 0)
    (bind _returnvalue_4 (`PixelStreamingBlueprints.GetPixelStreamingDelegates`))
    (add `PixelStreamingDelegates.OnClosedConnection` _returnvalue_4 (delegate `Reset`))))

(event `OnBlueprintSignalling_Event` :!signature `self.OnBlueprintSignalling`
  (params (Signal :type "EBlueprintSignalling Enum" :default "SwitchToSceneCam"))
  (`self.HandleBlueprintSignal` Signal))

(event `OnPixelStreamingResponse_Event` :!signature `self.OnPixelStreamingResponse`
  (params (Message :type String))
  (`self.HandleResponding` Message))

(event `Reset`
  (params (StreamerId :type String) (PlayerId :type String) (WasQualityController :type Boolean))
  (`self.ResetSynavisState`))

(event `self.PixelStreamingInput.OnInputEvent`
  (params (Descriptor :type String))
  (`self.ParseInput` Descriptor))

(event `OnPixelStreamingGeometry_Event` :!signature `self.OnPixelStreamingGeometry`
  (params (Points :type "Array of Vector Structure (by ref)") (Normals :type "Array of Vector Structure (by ref)") (Triangles :type "Array of Integer (by ref)") (TexCoords :type "Array of Vector2D Structure (by ref)") (Values :type "Array of Float (single-precision) (by ref)") (Time :type "Float (single-precision)"))
  (`self.HandleGeometrySpawn` Points Triangles Normals TexCoords Time Values))

(fn `HandleBlueprintSignal`
  (params (Enumerator :type "EBlueprintSignalling Enum" :default "SwitchToSceneCam"))
  (switch `EBlueprintSignalling` Enumerator
    (:`SwitchToSceneCam`
      (`Widget.RemoveFromParent` (`self.DualOverlay`))
      (`UserWidget.AddToViewport` (`self.SingleOverlay`) 0)
      (`/SynavisUE/SingleView.ChangeTarget` (`self.SingleOverlay`) 1))
    (:`SwitchToInfoCam`
      (`Widget.RemoveFromParent` (`self.DualOverlay`))
      (`ActorComponent.Activate` (`self.InfoCam`) true)
      (`/SynavisUE/SingleView.ChangeTarget` (`self.SingleOverlay`) 0))
    (:`SwitchToBothCams`
      (`Widget.RemoveFromParent` (`self.SingleOverlay`))
      (`UserWidget.AddToViewport` (`self.DualOverlay`) 0)
      (`self.SetActorHiddenInGame` (`Controller.K2_GetPawn` (`GameplayStatics.GetPlayerControllerFromID` 0)) true))))

(fn `HandleGeometrySpawn`
  (params (Vertices :type "Array of Vector Structure (by ref)") (Triangles :type "Array of Integer (by ref)") (Normals :type "Array of Vector Structure (by ref)") (UV0 :type "Array of Vector2D Structure (by ref)") (Time :type "Float (double-precision)") (Values :type "Array of Float (double-precision)"))
  (bind _returnvalue (`|SpawnActorFromClass` "/Script/Engine.Actor" (`KismetMathLibrary.MakeTransform` (0.0 0.0 0.0) (`KismetMathLibrary.RandomRotator` false)) "Undefined" "OverrideRootScale" self null))
  (bind _returnvalue_2 (`AddComponent|NODE_AddProceduralMeshComponent-0` :`self` _returnvalue))
  (`ProceduralMeshComponent.ClearAllMeshSections` _returnvalue_2)
  (`ProceduralMeshComponent.CreateMeshSection_LinearColor` :`self` _returnvalue_2 :`Vertices` Vertices :`Triangles` Triangles :`Normals` Normals :`UV0` UV0)
  (`PrimitiveComponent.SetMaterial` _returnvalue_2 0 null))

(fn `HandleResponding`
  (params (InString :type String))
  (`PixelStreamingInput.SendPixelStreamingResponse` (`self.PixelStreamingInput`) InString))

(fn `UserConstructionScript`)